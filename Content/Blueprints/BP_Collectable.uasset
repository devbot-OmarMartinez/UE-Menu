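; BP_Collectable is a collectable actor that the third-person character picks up by touch.
; On BeginPlay it looks up its Type enum as a row name in the collectibles DataTable and shows that row's Title in its CollectableName text.
; When its Collision component overlaps a BP_ThirdPersonCharacter, it passes Type to that character's NewCollectable.
; The actor does not destroy or hide itself in this graph.
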(event `self.ReceiveBeginPlay`
  (bind _returnvalue (`|GetDataTableRow` "/Game/Data/CollectiblesDataTable.CollectiblesDataTable" (`KismetStringLibrary.Conv_StringToName` (`|GetEnumeratorNameAsString` (`self.Type`))))
    (:`then`
      (bind _output_get (set `self.SelectedRow` _returnvalue))
      (`TextRenderComponent.K2_SetText` (`self.CollectableName`) (`KismetTextLibrary.Conv_StringToText` (`.Title_5_490A6B074BDF8AF29A8DE395153557F3` (break `/Game/Data/CollectibleDataStruct` _output_get)))))))

(event `self.Collision.OnComponentBeginOverlap`
  (params (OverlappedComponent :type "PrimitiveComponent Object Reference") (OtherActor :type "Actor Object Reference") (OtherComp :type "PrimitiveComponent Object Reference") (OtherBodyIndex :type Integer) (bFromSweep :type Boolean) (SweepResult :type "HitResult Structure (by ref)"))
  (bind _asbp_third_person_character (cast `/Game/ThirdPerson/Blueprints/BP_ThirdPersonCharacter` OtherActor))
  (`/Game/ThirdPerson/Blueprints/BP_ThirdPersonCharacter.NewCollectable` _asbp_third_person_character (`self.Type`)))

(fn `UserConstructionScript`)